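; Construction-script Blueprint that repeats a chosen static mesh along a circular arc to build a generic circular array.
; It adds one mesh component per item, placed by sine and cosine of an initial angle plus a per-index angle step, at a set radius.
; The circle is shifted back by that radius on Y, and each copy is yawed by the negated angle to follow the curve.
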(fn `UserConstructionScript`
  (bind _distance (`self.Distance`))
  (for _index (range 1 (+ (`self.NumItems`) 1))
    (bind _returnvalue (+ (* _index (`self.DeltaAngle`)) (`self.InitialAngle`)))
    (bind _returnvalue_2 (`AddComponent|StaticMeshComponent_482` :`RelativeTransform` (`KismetMathLibrary.MakeTransform` (`KismetMathLibrary.MakeVector` (* (`KismetMathLibrary.DegSin` _returnvalue) _distance) (- (* (`KismetMathLibrary.DegCos` _returnvalue) _distance) _distance)) (`KismetMathLibrary.NegateRotator` (`KismetMathLibrary.MakeRotator` 0.0 0.0 _returnvalue)))))
    (if (!= (`self.StaticMeshToRepeat`) null)
      (`StaticMeshComponent.SetStaticMesh` _returnvalue_2 (`self.StaticMeshToRepeat`))
      (`PrimitiveComponent.SetCastShadow` _returnvalue_2 true)
      (`PrimitiveComponent.SetEnableGravity` _returnvalue_2 false))))