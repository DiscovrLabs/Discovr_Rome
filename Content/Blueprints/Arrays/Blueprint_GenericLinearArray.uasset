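; Generic linear array Blueprint that repeats one static mesh in an evenly spaced line.
; The Construction Script adds NumItems static mesh components, each offset by a multiple of Distance and sharing the internal X, Y and Z scale.
; When StaticMeshToRepeat is set, each component gets that mesh with shadows on and gravity off, plus MaterialToUse in slot 0 if provided.
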(fn `UserConstructionScript`
  (for _index (range 1 (+ (`self.NumItems`) 1))
    (bind _returnvalue (`AddComponent|Static Mesh Component_987` :`RelativeTransform` (`KismetMathLibrary.MakeTransform` (* (`self.Distance`) (`KismetMathLibrary.Conv_IntToDouble` (- _index 1))) (struct) (`KismetMathLibrary.MakeVector` (`self.InternalScaleX`) (`self.InternalScaleY`) (`self.InternalScaleZ`)))))
    (if (!= (`self.StaticMeshToRepeat`) null)
      (`StaticMeshComponent.SetStaticMesh` _returnvalue (`self.StaticMeshToRepeat`))
      (`PrimitiveComponent.SetCastShadow` _returnvalue true)
      (`PrimitiveComponent.SetEnableGravity` _returnvalue false)
      (if (!= (`self.MaterialToUse`) null)
        (`PrimitiveComponent.SetMaterial` _returnvalue 0 (`self.MaterialToUse`))))))