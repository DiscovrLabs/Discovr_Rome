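; Construction-script Blueprint that builds a rectangular 3D grid of repeated static meshes.
; Three nested loops over the X, Y and Z counts add a mesh component per cell, offset by per-axis spacing and given a shared scale.
; When a mesh is set, each component receives it with shadow casting on and gravity off, plus an optional material override on slot 0.
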(fn `UserConstructionScript`
  (for _index (range 1 (+ (`self.NumItemsX`) 1))
    (for _index_2 (range 1 (+ (`self.NumItemsY`) 1))
      (for _index_3 (range 1 (+ (`self.NumItemsZ`) 1))
        (bind _returnvalue (`AddComponent|StaticMeshComponent_1999` :`RelativeTransform` (`KismetMathLibrary.MakeTransform` (`KismetMathLibrary.MakeVector` (* (- _index 1) (`self.DistanceX`)) (* (- _index_2 1) (`self.DistanceY`)) (* (- _index_3 1) (`self.DistanceZ`))) (struct) (`KismetMathLibrary.MakeVector` (`self.InternalScaleX`) (`self.InternalScaleY`) (`self.InternalScaleZ`)))))
        (if (!= (`self.StaticMeshToRepeat`) null)
          (`StaticMeshComponent.SetStaticMesh` _returnvalue (`self.StaticMeshToRepeat`))
          (`PrimitiveComponent.SetCastShadow` _returnvalue true)
          (`PrimitiveComponent.SetEnableGravity` _returnvalue false)
          (if (!= (`self.MaterialToUse`) null)
            (`PrimitiveComponent.SetMaterial` _returnvalue 0 (`self.MaterialToUse`))))))))