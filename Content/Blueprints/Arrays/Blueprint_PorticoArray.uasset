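; Procedural portico builder that lays out a rectangular ring of arches, sized by NumItemsX, NumItemsY and ArchDistance.
; The construction script walks four sides, adding static mesh and box collision components for arches, the points between them, and corners.
; Helper functions derive each piece's position and 90-degree yaw step from side and order index.
; IsExterior selects between parallel component branches for in-between and corner pieces.
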(fn `GetArchRelativeTransform`
  (params (SideIndex :type Integer) (OrderIndex :type Integer))
  (returns (ArchRelativeTransform :type "Object.Transform Structure") (CollisionRelativeTransform :type "Object.Transform Structure"))
  (bind _archdistance (`self.ArchDistance`))
  (bind _archdistance_2 (`self.ArchDistance`))
  (bind _archdistance_3 (`self.ArchDistance`))
  (bind _returnvalue (`KismetMathLibrary.MakeRot` 0.0 (`self.Rotation`)))
  (bind _returnvalue_2 (* (- OrderIndex 1) _archdistance_3))
  (bind _returnvalue_3 (- _returnvalue_2 (/ _archdistance_3 2.0)))
  (set `self.Rotation` (* (- SideIndex 1) 90.0))
  (if (== SideIndex 1)
    (set `self.SideOffsetY` 0.0)
    (set `self.SideOffsetX` 0.0)
    (set `self.ArchOffsetY` _returnvalue_2)
    (set `self.ArchOffsetX` 0.0)
    (set `self.CollisionOffsetY` _returnvalue_3)
    (set `self.CollisionOffsetX` 0.0)
    (elif (== SideIndex 2)
      (set `self.SideOffsetY` (* (- (`KismetMathLibrary.Conv_IntToDouble` (`self.NumItemsY`)) 0.5) _archdistance_2))
      (set `self.SideOffsetX` (/ _archdistance_2 -2.0))
      (set `self.ArchOffsetY` 0.0)
      (set `self.ArchOffsetX` (* _returnvalue_2 -1.0))
      (set `self.CollisionOffsetY` 0.0)
      (set `self.CollisionOffsetX` (* _returnvalue_3 -1.0))
      (elif (== SideIndex 3)
        (set `self.SideOffsetY` (* (- (`KismetMathLibrary.Conv_IntToDouble` (`self.NumItemsY`)) 1.0) _archdistance))
        (set `self.SideOffsetX` (* (* _archdistance (`KismetMathLibrary.Conv_IntToDouble` (`self.NumItemsX`))) -1.0))
        (set `self.ArchOffsetY` (* _returnvalue_2 -1.0))
        (set `self.ArchOffsetX` 0.0)
        (set `self.CollisionOffsetY` (* _returnvalue_3 -1.0))
        (set `self.CollisionOffsetX` 0.0)
        (elif (== SideIndex 4)
          (set `self.SideOffsetY` (/ (`self.ArchDistance`) -2.0))
          (set `self.SideOffsetX` (* (* (- (`KismetMathLibrary.Conv_IntToDouble` (`self.NumItemsX`)) 0.5) (`self.ArchDistance`)) -1.0))
          (set `self.ArchOffsetY` 0.0)
          (set `self.ArchOffsetX` _returnvalue_2)
          (set `self.CollisionOffsetY` 0.0)
          (set `self.CollisionOffsetX` _returnvalue_3)))))
  (return (`KismetMathLibrary.MakeTransform` (`KismetMathLibrary.MakeVector` (+ (`self.SideOffsetX`) (`self.ArchOffsetX`)) (+ (`self.SideOffsetY`) (`self.ArchOffsetY`))) _returnvalue) (`KismetMathLibrary.MakeTransform` (`KismetMathLibrary.MakeVector` (+ (`self.SideOffsetX`) (`self.CollisionOffsetX`)) (+ (`self.SideOffsetY`) (`self.CollisionOffsetY`)) 0.0) _returnvalue)))

(fn `GetCornersRelativeTransform`
  (params (SideIndex :type Integer))
  (returns (CornerRelativeTransform :type "Object.Transform Structure") (CollisionRelativeTransform :type "Object.Transform Structure"))
  (bind _cornercollisionoffset (`self.CornerCollisionOffset`))
  (bind _cornercollisionoffset_2 (`self.CornerCollisionOffset`))
  (bind _cornercollisionoffset_3 (`self.CornerCollisionOffset`))
  (bind _returnvalue (`KismetMathLibrary.MakeRot` 0.0 (`self.Rotation`)))
  (bind _returnvalue_2 (/ (`self.ArchDistance`) -2.0))
  (bind _returnvalue_3 (- _returnvalue_2 _cornercollisionoffset))
  (bind _returnvalue_4 (* (- (`KismetMathLibrary.Conv_IntToDouble` (`self.NumItemsY`)) 0.5) (`self.ArchDistance`)))
  (bind _returnvalue_5 (* (* (`KismetMathLibrary.Conv_IntToDouble` (`self.NumItemsX`)) (`self.ArchDistance`)) -1.0))
  (set `self.Rotation` (* (- SideIndex 1) 90.0))
  (if (== SideIndex 1)
    (set `self.SideOffsetY` _returnvalue_4)
    (set `self.SideOffsetX` 0.0)
    (set `self.CollisionOffsetY` (+ _returnvalue_4 _cornercollisionoffset_2))
    (set `self.CollisionOffsetX` _cornercollisionoffset_2)
    (return (`KismetMathLibrary.MakeTransform` (`KismetMathLibrary.MakeVector` (`self.SideOffsetX`) (`self.SideOffsetY`)) _returnvalue) (`KismetMathLibrary.MakeTransform` (`KismetMathLibrary.MakeVector` (`self.CollisionOffsetX`) (`self.CollisionOffsetY`) 0.0) _returnvalue))
    (elif (== SideIndex 2)
      (set `self.SideOffsetY` _returnvalue_4)
      (set `self.SideOffsetX` _returnvalue_5)
      (set `self.CollisionOffsetY` (+ _returnvalue_4 _cornercollisionoffset_3))
      (set `self.CollisionOffsetX` (- _returnvalue_5 _cornercollisionoffset_3))
      (return (`KismetMathLibrary.MakeTransform` (`KismetMathLibrary.MakeVector` (`self.SideOffsetX`) (`self.SideOffsetY`)) _returnvalue) (`KismetMathLibrary.MakeTransform` (`KismetMathLibrary.MakeVector` (`self.CollisionOffsetX`) (`self.CollisionOffsetY`) 0.0) _returnvalue))
      (elif (== SideIndex 3)
        (set `self.SideOffsetY` _returnvalue_2)
        (set `self.SideOffsetX` _returnvalue_5)
        (set `self.CollisionOffsetY` _returnvalue_3)
        (set `self.CollisionOffsetX` (- _returnvalue_5 _cornercollisionoffset))
        (return (`KismetMathLibrary.MakeTransform` (`KismetMathLibrary.MakeVector` (`self.SideOffsetX`) (`self.SideOffsetY`)) _returnvalue) (`KismetMathLibrary.MakeTransform` (`KismetMathLibrary.MakeVector` (`self.CollisionOffsetX`) (`self.CollisionOffsetY`) 0.0) _returnvalue))
        (elif (== SideIndex 4)
          (set `self.SideOffsetY` _returnvalue_2)
          (set `self.SideOffsetX` 0.0)
          (set `self.CollisionOffsetY` _returnvalue_3)
          (set `self.CollisionOffsetX` _cornercollisionoffset)
          (return (`KismetMathLibrary.MakeTransform` (`KismetMathLibrary.MakeVector` (`self.SideOffsetX`) (`self.SideOffsetY`)) _returnvalue) (`KismetMathLibrary.MakeTransform` (`KismetMathLibrary.MakeVector` (`self.CollisionOffsetX`) (`self.CollisionOffsetY`) 0.0) _returnvalue)))))))

(fn `UserConstructionScript`
  (for _index (range 1 5)
    (if (== _index 1)
      (set `self.SideNumItems` (`self.NumItemsY`) :!label _label)
      (for _index_2 (range 1 (+ (`self.SideNumItems`) 1)) :!label _label_2
        (bind (_archrelativetransform _collisionrelativetransform) (`self.GetArchRelativeTransform` _index _index_2))
        (`AddComponent|StaticMeshComponent_1935` :`RelativeTransform` _archrelativetransform)
        (bind _outtransform (`self.OffsetTransform` _collisionrelativetransform))
        (`AddComponent|BoxComponent_380` :`RelativeTransform` _outtransform)
        (if (!= _index_2 1)
          (if (`self.IsExterior`)
            (`AddComponent|StaticMeshComponent_19493` :`RelativeTransform` _collisionrelativetransform)
            (`AddComponent|BoxComponent_14056` :`RelativeTransform` _outtransform)
            (else
              (`AddComponent|StaticMeshComponent_24617` :`RelativeTransform` _collisionrelativetransform)
              (`AddComponent|BoxComponent_14057` :`RelativeTransform` _outtransform)))))
      (bind (_cornerrelativetransform _collisionrelativetransform_2) (`self.GetCornersRelativeTransform` _index))
      (if (`self.IsExterior`)
        (`AddComponent|StaticMeshComponent_6807` :`RelativeTransform` _cornerrelativetransform)
        (bind _outtransform_2 (`self.OffsetTransform` _collisionrelativetransform_2))
        (`AddComponent|BoxComponent_602` :`RelativeTransform` _outtransform_2)
        (else
          (`AddComponent|StaticMeshComponent_32090` :`RelativeTransform` _cornerrelativetransform)
          (`AddComponent|BoxComponent_20186` :`RelativeTransform` _outtransform_2)))
      (elif (== _index 2)
        (set `self.SideNumItems` (`self.NumItemsX`) :!label _label_3)
        (goto _label_2)
        (elif (== _index 3)
          (goto _label)
          (elif (== _index 4)
            (goto _label_3)))))))