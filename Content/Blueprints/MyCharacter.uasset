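; Character Blueprint that adds footstep and landing audio to the player or pawn's movement.
; A randomized Delay on Tick acts as a repeating step timer, playing the footstep cue below the actor when it is walking above a small horizontal speed.
; On landing, the same cue plays twice in quick succession, louder and lower-pitched, to suggest a heavier impact.
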(event `self.ReceiveTick`
  (params (DeltaSeconds :type "Float (single-precision)"))
  (bind _charactermovement (`self.CharacterMovement`))
  (bind _velocity (`MovementComponent.Velocity` _charactermovement))
  ;[1 1 1] Plays footstep sounds  when walking around
  (`KismetSystemLibrary.Delay` (`KismetMathLibrary.RandomFloatInRange` 0.45 0.55)) ; Footstep interval
  (if (and (`|EnumEquality` (`CharacterMovementComponent.MovementMode` _charactermovement) "MOVE_Walking") (> (`KismetMathLibrary.VSize` (* _velocity (1.0 1.0 0.0))) 50.0))
    (`GameplayStatics.PlaySoundAtLocation` "/Game/Audio/Blueprints_Footstep_Cue.Blueprints_Footstep_Cue" (+ (- (`self.K2_GetActorLocation`) (0.0 0.0 80.0)) (* (`KismetMathLibrary.Normal` _velocity) 0.0)) (struct) 0.7)))

(event `self.OnLanded`
  (params (Hit :type "HitResult Structure (by ref)"))
  (bind _returnvalue (- (`self.K2_GetActorLocation`) (0.0 0.0 80.0)))
  ;[1 1 1] Plays sounds after character was jumping or falling
  (`GameplayStatics.PlaySoundAtLocation` "/Game/Audio/Blueprints_Footstep_Cue.Blueprints_Footstep_Cue" _returnvalue (struct) 1.6 0.8)
  (`KismetSystemLibrary.Delay` 0.07)
  (`GameplayStatics.PlaySoundAtLocation` "/Game/Audio/Blueprints_Footstep_Cue.Blueprints_Footstep_Cue" _returnvalue (struct) 1.5 0.7))

(fn `UserConstructionScript`)